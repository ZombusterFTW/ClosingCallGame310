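; BatteryManager is a Blueprint that switches all flashlight battery pickups in the level on or off together.
; On BeginPlay it gathers every Flashlight_Battery_Pickup actor into the LevelBatteries array.
; Its EnableBatteries and DisableBatteries events loop over that cached array, call the matching event on each pickup, and print a debug message.
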(event Custom|EnableBatteries
  (for _array_element (Variables|Default|GetLevelBatteries)
    (Default|EnableBattery _array_element))
  (Development|PrintString "Enabled All Batteries"))

(event Custom|DisableBatteries
  (for _array_element (Variables|Default|GetLevelBatteries)
    (Default|DisableBattery _array_element))
  (Development|PrintString "Disabled All Batteries"))

(event EventBeginPlay
  (bind _outactors (Actor|GetAllActorsOfClass "/Game/ClosingCall/Blueprints/Flashlight_Battery_Pickup.Flashlight_Battery_Pickup_C"))
  (Variables|Default|SetLevelBatteries _outactors))

(event Collision|EventActorBeginOverlap
  (params (OtherActor :type Actor%20Object%20Reference)))

(event EventTick
  (params (DeltaSeconds :type Float%20%28single-precision%29)))

(fn ConstructionScript)