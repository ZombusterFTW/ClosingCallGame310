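; Easter egg statue actor that, once activated, scolds the player for staring at it and sends them to Theatre 1.
; Tick uses a camera dot-product check and line trace to accumulate continuous looking time, resetting when the gaze breaks.
; Each threshold hit raises the next threshold, plays escalating dialogue and sets a goal widget; the third deactivates the statue.
; A per-tick delay loop awaits audio completion, calling the lobby trigger after the final count.
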(event Custom|Activate
  (Variables|Default|SetIsActive? true))

(event EventBeginPlay
  (bind _returnvalue (Actor|GetActorOfClass "/Game/FirstPerson/Blueprints/BP_FirstPersonCharacter.BP_FirstPersonCharacter_C"))
  (Variables|Default|SetPlayerRef _returnvalue))

(event Collision|EventActorBeginOverlap
  (params (OtherActor :type Actor%20Object%20Reference)))

(event EventTick
  (params (DeltaSeconds :type Float%20%28single-precision%29))
  (bind _lookingcount (Variables|Default|GetLookingCount))
  (bind _context (Variables|Default|GetContext))
  (bind _playerref (Variables|Default|GetPlayerRef))
  (if (Math|Boolean|ANDBoolean (CallFunction|IsPlayerLooking?) (not (Variables|Default|GetAudioPlaying?)) (Variables|Default|GetIsActive?))
    (bind _returnvalue (Utilities|PlayerCameraLineTrace 5e+03))
    (if _returnvalue
      (bind _output_get (Variables|Default|SetLookingTime (+ DeltaSeconds (Variables|Default|GetLookingTime))))
      (Development|PrintString "adding delta time" false)
      (if (>= _output_get (Variables|Default|GetTimeToLook))
        (bind _counter (Utilities|FlowControl|DoN _lookingcount)
          (:Exit
            (Variables|Default|SetLookingTime 0.0)
            (Variables|Default|SetTimeToLook (+ (Variables|Default|GetTimeToLook) (Variables|Default|GetAddTimeEachTime)))
            (Variables|Default|SetAudioPlaying? true)
            (switch int (- _counter 1)
              (:Default
                (Development|PrintString "StatueStareEEOutOFBounds"))
              (:0
                (Utilities|FlowControl|Sequence
                  (:then_0
                    (bind _returnvalue_2 (Class|GameplayStatics|SpawnDialogueatLocation "/Game/ClosingCall/VO/Dialouge/StatueStareEE1_Dialogue.StatueStareEE1_Dialogue" _context "0, 0, 0" "0, 0, 0" 1.0 1.0 0.0 0 false))
                    (bind _output_get_2 (Variables|Default|SetPlayingAudio _returnvalue_2))
                    (Audio|Components|Audio|Play (stale _output_get_4) 0.0 :!label _label)
                    (Utilities|WhileLoopwithDelay (Audio|Components|Audio|IsPlaying (stale _output_get_3)) :!label _label_2
                      (:Loop%20Body
                        (Utilities|FlowControl|DelayUntilNextTick)
                        (goto _label_2 FromDelay))
                      (:Completed
                        (Variables|Default|SetAudioPlaying? false)
                        (if (== _counter _lookingcount)
                          (Default|CallStartLobbyTrigger)))))
                  (:then_1
                    (Default|CreateGoalUIWidget _playerref "Head To Theatre 1"))))
              (:1
                (Utilities|FlowControl|Sequence
                  (:then_0
                    (bind _returnvalue_3 (Class|GameplayStatics|SpawnDialogueatLocation "/Game/ClosingCall/VO/Dialouge/StatueStare2_Dialogue.StatueStare2_Dialogue" _context "0, 0, 0" "0, 0, 0" 1.0 1.0 0.0 0 false))
                    (bind _output_get_3 (Variables|Default|SetPlayingAudio _returnvalue_3))
                    (goto _label))
                  (:then_1
                    (Default|CreateGoalUIWidget _playerref "Stop Looking At The Statue. And Go To Theatre 1"))))
              (:2
                (Utilities|FlowControl|Sequence
                  (:then_0
                    (Variables|Default|SetIsActive? false)
                    (bind _returnvalue_4 (Class|GameplayStatics|SpawnDialogueatLocation "/Game/ClosingCall/VO/Dialouge/StatueStare3_Dialogue.StatueStare3_Dialogue" _context "0, 0, 0" "0, 0, 0" 1.0 1.0 0.0 0 false))
                    (bind _output_get_4 (Variables|Default|SetPlayingAudio _returnvalue_4))
                    (goto _label))
                  (:then_1
                    (Default|CreateGoalUIWidget _playerref "GO TO THEATRE 1 NOW. NO PLAYING AROUND -Supervisor"))))))))
      (else
        (Variables|Default|SetLookingTime 0.0)))
    (else
      (Variables|Default|SetLookingTime 0.0))))

(fn ConstructionScript)

(fn IsPlayerLooking?
  (return (> (Class|Actor|GetDotProductto (Game|GetPlayerCameraManager 0) self) 0.0)))