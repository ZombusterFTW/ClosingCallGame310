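; Interactable computer in the Theatre 3 reset puzzle that the player must restart, then confirm, before timeouts fail it.
; StartPC flashes purple after a random delay; Use starts a timed yellow reset, then blue flashing awaits confirmation, which turns it green.
; It reports activation, lock-in and failure to the Theatre3Switch actor found at BeginPlay.
; Monitor material swaps show state; overlap shows prompts, and Tick enables input only while overlapped and active.
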(event OnComponentBeginOverlap(ComputerTrigger)
  (params (OverlappedComponent :type Primitive%20Component%20Object%20Reference) (OtherActor :type Actor%20Object%20Reference) (OtherComp :type Primitive%20Component%20Object%20Reference) (OtherBodyIndex :type Integer) (bFromSweep :type Boolean) (SweepResult :type Hit%20Result%20Structure%20%28by%20ref%29))
  ;[1 0 0] Detect Overlap and Create UI if needed
  (Utilities|Casting|CastToBP_FirstPersonCharacter OtherActor)
  (Variables|Default|SetIsOverlappingComputer? true)
  (if (Variables|Default|GetIsActive?)
    (if (Variables|Default|GetReadyToConfirm?)
      (Utilities|IsValid (Variables|Default|GetPickupPrompt)
        (:Is%20Not%20Valid
          (bind _returnvalue (UserInterface|CreateWidget "/Game/ClosingCall/UI/PickupPrompt.PickupPrompt_C"))
          (bind _output_get (Variables|Default|SetPickupPrompt _returnvalue))
          (Variables|/Game/ClosingCall/UI/PickupPrompt.PickupPrompt_C|SetPromptText _output_get (Utilities|Text|ToText(String) (Variables|Default|GetComputerHintTextConfirm)))
          (UserInterface|Viewport|AddtoViewport _output_get 0)))
      (else
        (Utilities|IsValid (Variables|Default|GetPickupPrompt)
          (:Is%20Not%20Valid
            (bind _returnvalue_2 (UserInterface|CreateWidget "/Game/ClosingCall/UI/PickupPrompt.PickupPrompt_C"))
            (bind _output_get_2 (Variables|Default|SetPickupPrompt _returnvalue_2))
            (Variables|/Game/ClosingCall/UI/PickupPrompt.PickupPrompt_C|SetPromptText _output_get_2 (Utilities|Text|ToText(String) (Variables|Default|GetComputerHintText)))
            (UserInterface|Viewport|AddtoViewport _output_get_2 0)))))))

(event OnComponentEndOverlap(ComputerTrigger)
  (params (OverlappedComponent :type Primitive%20Component%20Object%20Reference) (OtherActor :type Actor%20Object%20Reference) (OtherComp :type Primitive%20Component%20Object%20Reference) (OtherBodyIndex :type Integer))
  ;[1 0 0] Detect Overlap and Create UI if needed
  (Utilities|Casting|CastToBP_FirstPersonCharacter OtherActor)
  (Variables|Default|SetIsOverlappingComputer? false)
  (Utilities|IsValid (Variables|Default|GetPickupPrompt)
    (:Is%20Valid
      (Widget|RemovefromParent (Variables|Default|GetPickupPrompt))
      (Variables|Default|SetPickupPrompt 0))))

(event Custom|GetComputerIndex
  (params (Index :type Integer))
  ;[0.9882 1 0] Get Computer Index For Hint String DEBUG
)

(event Custom|StartPC
  ;[1 1 1] StartPC
  (Variables|Default|SetCompleted? false)
  (Variables|Default|SetFailed? false)
  (Utilities|FlowControl|Delay (Math|Random|RandomFloatinRange (Variables|Default|GetMinTimeTillNextPC) (Variables|Default|GetMaxTimeTillNextPC)))
  (Variables|Default|SetIsActive? false)
  (Variables|Default|SetLightCycling? true)
  (Utilities|FlowControl|Sequence
    (:then_0
      (Utilities|WhileLoopwithDelay (Variables|Default|GetLightCycling?) :!label _label
        (:LoopBody
          (Utilities|FlashColor "/Game/ClosingCall/ModelsandAssets/Materials/Purple_Simon.Purple_Simon" (Variables|Default|GetLightCycling?))
          (Variables|Default|SetIsActive? true)
          (goto _label FromDelay))))
    (:then_1
      (Utilities|FlowControl|Delay (Variables|Default|GetPCWaitingToStartResetTimeOut))
      (if (not (Variables|Default|GetIsReseting?))
        (if (not (or (Variables|Default|GetFailed?) (Variables|Default|GetCompleted?)))
          (Development|PrintString "PC Waited For Too Long To Start Restart. Fail")
          (Default|PCFailed (Variables|Default|GetParentSwitch)))))))

(event Custom|TurnOff
  ;[1 1 1] Turn Off PC
  (Rendering|Material|SetMaterial (Variables|Debug|GetStaticMeshComponent) 1 "/Game/HB_ComputersPack/Materials/MI_LCDMonitorB.MI_LCDMonitorB")
  (Variables|Default|SetIsActive? false)
  (Variables|Default|SetIsReseting? false)
  (Variables|Default|SetReadyToConfirm? false)
  (Variables|Default|SetConfirmed? false))

(event Custom|PCReadyToConfirm
  ;[1 1 1] PC Flash when ready to confirm
  (Variables|Default|SetIsActive? false)
  (Variables|Default|SetLightCycling? true)
  (Utilities|WhileLoopwithDelay (Variables|Default|GetLightCycling?) :!label _label
    (:LoopBody
      (Utilities|FlashColor "/Game/ClosingCall/ModelsandAssets/Materials/Blue_Simon_Inst.Blue_Simon_Inst" (Variables|Default|GetLightCycling?))
      (Variables|Default|SetIsActive? true)
      (goto _label FromDelay))))

(event Custom|PCFailed
  ;[1 1 1] Fail Event
  (Variables|Default|SetFailed? true)
  (Variables|Default|SetIsActive? false)
  (Variables|Default|SetIsReseting? false)
  (Variables|Default|SetReadyToConfirm? false)
  (Variables|Default|SetConfirmed? false))

(event Custom|CompletedSequence
  ;[1 1 1] Set Bool To Prevent Fail if player wins too fast.
  (Variables|Default|SetCompleted? true))

(event EventBeginPlay
  ;[1 1 1] Begin Play
  (Utilities|FlowControl|Sequence
    (:then_0
      (bind _returnvalue (Actor|GetActorOfClass "/Game/ClosingCall/Blueprints/Theatre3Switch_ComputerReset_ClosingCall.Theatre3Switch_ComputerReset_ClosingCall_C"))
      (Variables|Default|SetParentSwitch _returnvalue)
      (Variables|Default|SetComputerModel (Variables|Debug|GetStaticMeshComponent)))))

(event EventTick
  (params (DeltaSeconds :type Float%20%28single-precision%29))
  (bind _returnvalue (Game|GetPlayerController 0))
  (Utilities|FlowControl|Sequence
    (:then_0
      ;[1 1 1] Enable Input on Overlap
      (if (and (Variables|Default|GetIsOverlappingComputer?) (Variables|Default|GetIsActive?))
        (Input|EnableInput _returnvalue)
        (else
          (Input|DisableInput _returnvalue))))))

(event Input|ActionEvents|InputActionUse/Pickup
  (params (Key :type Key%20Structure :default "None"))
  ;[1 1 1] Confirm PC Interact
  (:Pressed
    (if (and (Variables|Default|GetReadyToConfirm?) (Variables|Default|GetIsReseting?))
      (Variables|Default|SetLightCycling? false)
      (Variables|Default|SetIsActive? false)
      (Utilities|FlowControl|Delay 0.3)
      (Utilities|FlashColor "/Game/ClosingCall/ModelsandAssets/Materials/Green_Simon.Green_Simon" (not (Variables|Default|GetFailed?)))
      (Utilities|FlowControl|Delay 0.3)
      (Rendering|Material|SetMaterial (Variables|Debug|GetStaticMeshComponent) 1 "/Game/ClosingCall/ModelsandAssets/Materials/Green_Simon.Green_Simon")
      (Variables|Default|SetConfirmed? true)
      (Development|PrintString "Reset Confiirmed")
      (Default|PCLockedin (Variables|Default|GetParentSwitch)))))

(event Input|ActionEvents|InputActionUse/Pickup
  (params (Key :type Key%20Structure :default "None"))
  (bind _parentswitch (Variables|Default|GetParentSwitch))
  ;[1 1 1] First Interact to start the restart
  (:Pressed
    (if (and (not (Variables|Default|GetIsReseting?)) (Variables|Default|GetIsActive?))
      (Variables|Default|SetLightCycling? false)
      (Variables|Default|SetIsActive? false)
      (Utilities|FlowControl|Delay 0.3)
      (Utilities|FlashColor "/Game/ClosingCall/ModelsandAssets/Materials/Yellow_Simon.Yellow_Simon" (not (Variables|Default|GetFailed?)))
      (Default|PCActivated _parentswitch)
      (Rendering|Material|SetMaterial (Variables|Debug|GetStaticMeshComponent) 1 "/Game/ClosingCall/ModelsandAssets/Materials/Yellow_Simon.Yellow_Simon")
      (Variables|Default|SetIsReseting? true)
      (Utilities|FlowControl|Delay (Math|Random|RandomFloatinRange (Variables|Default|GetMinResetTime) (Variables|Default|GetMaxResetTime)))
      (if (not (Variables|Default|GetFailed?))
        (CallFunction|PCReadytoConfirm)
        (Variables|Default|SetReadyToConfirm? true)
        (Utilities|FlowControl|Delay (Variables|Default|GetTimeAfterReset))
        (if (not (Math|Boolean|ORBoolean (Variables|Default|GetConfirmed?) (Variables|Default|GetCompleted?) (Variables|Default|GetFailed?)))
          (Default|PCFailed _parentswitch)
          (Development|PrintString "Reset Was Not Confirmed In Time Fail."))))))

(fn ConstructionScript)