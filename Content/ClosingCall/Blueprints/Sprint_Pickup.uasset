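; A sprite pickup that grants the first-person character the sprint ability and rotates each tick to stay aligned with the player camera.
; HitBox overlap shows or removes a prompt widget and sets a flag that Tick uses to enable or disable the pickup's input.
; Pressing Use/Pickup shows a fading "full" hint if sprint is already granted; otherwise it grants sprint, shows controls, fires a pickup event and destroys itself.
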(event OnComponentBeginOverlap(HitBox)
  (params (OverlappedComponent :type Primitive%20Component%20Object%20Reference) (OtherActor :type Actor%20Object%20Reference) (OtherComp :type Primitive%20Component%20Object%20Reference) (OtherBodyIndex :type Integer) (bFromSweep :type Boolean) (SweepResult :type Hit%20Result%20Structure%20%28by%20ref%29))
  ;[1 1 1] Pickup UI
  (Utilities|Casting|CastToBP_FirstPersonCharacter OtherActor)
  (Variables|Default|SetIsOverlap? true)
  (Utilities|IsValid (Variables|Default|GetPickupPrompt)
    (:Is%20Not%20Valid
      (bind _returnvalue (UserInterface|CreateWidget "/Game/ClosingCall/UI/PickupPrompt.PickupPrompt_C"))
      (bind _output_get (Variables|Default|SetPickupPrompt _returnvalue))
      (Variables|/Game/ClosingCall/UI/PickupPrompt.PickupPrompt_C|SetPromptText _output_get (Variables|Default|GetPromptText))
      (UserInterface|Viewport|AddtoViewport _output_get 0))))

(event OnComponentEndOverlap(HitBox)
  (params (OverlappedComponent :type Primitive%20Component%20Object%20Reference) (OtherActor :type Actor%20Object%20Reference) (OtherComp :type Primitive%20Component%20Object%20Reference) (OtherBodyIndex :type Integer))
  ;[1 1 1] Pickup UI
  (Utilities|Casting|CastToBP_FirstPersonCharacter OtherActor)
  (Variables|Default|SetIsOverlap? false)
  (Utilities|IsValid (Variables|Default|GetPickupPrompt)
    (:Is%20Valid
      (Widget|RemovefromParent (Variables|Default|GetPickupPrompt))
      (Variables|Default|SetPickupPrompt 0))))

(event EventBeginPlay
  (Utilities|FlowControl|Sequence))

(event EventTick
  (params (DeltaSeconds :type Float%20%28single-precision%29))
  (bind _returnvalue (Game|GetPlayerController 0))
  ;[1 1 1] Overlap Check
  (Utilities|FlowControl|Sequence
    (:then_0
      (if (Variables|Default|GetIsOverlap?)
        (Input|EnableInput _returnvalue)
        (else
          (Input|DisableInput _returnvalue))))
    (:then_1
      ;[1 1 1] Always face player
      (Transformation|SetActorRotation (Math|Rotator|MakeRotfromX (- (Transformation|GetWorldLocation (Variables|Default|GetSprintPickupSprite)) (Transformation|GetActorLocation (Game|GetPlayerCameraManager 0)))) true))))

(event Input|ActionEvents|InputActionUse/Pickup
  (params (Key :type Key%20Structure :default "None"))
  ;[1 1 1] Pickup Item
  (:Pressed
    (if (Variables|Default|GetIsOverlap?)
      (bind _asbp_first_person_character (Utilities|Casting|CastToBP_FirstPersonCharacter (Game|Player|GetPlayerPawn 0)))
      (if (Variables|/Game/FirstPerson/Blueprints/BP_FirstPersonCharacter.BP_FirstPersonCharacter_C|GetSprintGranted? _asbp_first_person_character)
        (Utilities|IsValid (Variables|Default|GetSprintFullUIHint)
          (:Is%20Not%20Valid
            (bind _returnvalue (UserInterface|CreateWidget "/Game/ClosingCall/UI/PlayerHint.PlayerHint_C"))
            (bind _output_get (Variables|Default|SetSprintFullUIHint _returnvalue))
            (Variables|/Game/ClosingCall/UI/PlayerHint.PlayerHint_C|SetPromptText _output_get (Variables|Default|GetPlayerFullPrompt))
            (UserInterface|Viewport|AddtoViewport _output_get 0)
            (UserInterface|Animation|PlayAnimation _output_get (Variables|/Game/ClosingCall/UI/PlayerHint.PlayerHint_C|GetFadeOut _output_get) 0.0 1 "Forward" 1.0 false)
            (Utilities|FlowControl|Delay 5.0)
            (Widget|RemovefromParent _output_get)
            (Variables|Default|SetSprintFullUIHint 0)))
        (else
          (Default|GrantSprint _asbp_first_person_character)
          (bind _returnvalue_2 (UserInterface|CreateWidget "/Game/ClosingCall/UI/PlayerHint.PlayerHint_C"))
          (Variables|/Game/ClosingCall/UI/PlayerHint.PlayerHint_C|SetPromptText _returnvalue_2 "Press Shift While Moving To Sprint")
          (UserInterface|Viewport|AddtoViewport _returnvalue_2 0)
          (UserInterface|Animation|PlayAnimation _returnvalue_2 (Variables|/Game/ClosingCall/UI/PlayerHint.PlayerHint_C|GetFadeOut _returnvalue_2) 0.0 1 "Forward" 1.0 false)
          (Default|CallSprintPickupEvent)
          (Actor|DestroyActor)
          (Utilities|FlowControl|Delay 5.0)
          (Widget|RemovefromParent _returnvalue_2))))))

(fn ConstructionScript)