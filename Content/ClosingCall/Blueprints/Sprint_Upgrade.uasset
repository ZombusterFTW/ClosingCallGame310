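; Pickup actor that upgrades the first-person character's sprint duration when the player presses Use/Pickup within its hit box.
; Overlap shows a prompt widget, and Tick enables or disables input from the overlap flag.
; If sprint is granted and its duration differs, it applies the upgrade and destroys itself; otherwise it shows a fading hint.
; Several names and the missing-sprint message still say flashlight, and the upgrade hint's delayed removal follows DestroyActor.
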(event OnComponentBeginOverlap(HitBox)
  (params (OverlappedComponent :type Primitive%20Component%20Object%20Reference) (OtherActor :type Actor%20Object%20Reference) (OtherComp :type Primitive%20Component%20Object%20Reference) (OtherBodyIndex :type Integer) (bFromSweep :type Boolean) (SweepResult :type Hit%20Result%20Structure%20%28by%20ref%29))
  ;[1 1 1] Pickup UI
  (Utilities|Casting|CastToBP_FirstPersonCharacter OtherActor)
  (Variables|Default|SetIsOverlap? true)
  (Utilities|IsValid (Variables|Default|GetPickupPrompt)
    (:Is%20Not%20Valid
      (bind _returnvalue (UserInterface|CreateWidget "/Game/ClosingCall/UI/PickupPrompt.PickupPrompt_C"))
      (bind _output_get (Variables|Default|SetPickupPrompt _returnvalue))
      (Variables|/Game/ClosingCall/UI/PickupPrompt.PickupPrompt_C|SetPromptText _output_get (Variables|Default|GetPromptText))
      (UserInterface|Viewport|AddtoViewport _output_get 0))))

(event OnComponentEndOverlap(HitBox)
  (params (OverlappedComponent :type Primitive%20Component%20Object%20Reference) (OtherActor :type Actor%20Object%20Reference) (OtherComp :type Primitive%20Component%20Object%20Reference) (OtherBodyIndex :type Integer))
  ;[1 1 1] Pickup UI
  (Utilities|Casting|CastToBP_FirstPersonCharacter OtherActor)
  (Variables|Default|SetIsOverlap? false)
  (Utilities|IsValid (Variables|Default|GetPickupPrompt)
    (:Is%20Valid
      (Widget|RemovefromParent (Variables|Default|GetPickupPrompt))
      (Variables|Default|SetPickupPrompt 0))))

(event EventBeginPlay
  (Utilities|FlowControl|Sequence
    (:then_0
      ;[1 1 1] Sprint Duration Debug
      (if (Variables|Default|GetbDebugPrompt)
        (Variables|Default|SetPromptText (Utilities|Text|ToText(String) (Utilities|String|Append (Utilities|String|ToString(Text) (Variables|Default|GetPromptText)) " " (Utilities|String|Append (Utilities|String|ToString(Float) (Variables|Default|GetSprintUpgradeTime)) " Seconds"))))))))

(event EventTick
  (params (DeltaSeconds :type Float%20%28single-precision%29))
  (bind _returnvalue (Game|GetPlayerController 0))
  (Utilities|FlowControl|Sequence
    (:then_0
      ;[1 1 1] Overlap Check
      (if (Variables|Default|GetIsOverlap?)
        (Input|EnableInput _returnvalue)
        (else
          (Input|DisableInput _returnvalue))))))

(event Input|ActionEvents|InputActionUse/Pickup
  (params (Key :type Key%20Structure :default "None"))
  ;[1 1 1] Pickup Item
  (:Pressed
    (if (Variables|Default|GetIsOverlap?)
      (bind _asbp_first_person_character (Utilities|Casting|CastToBP_FirstPersonCharacter (Game|Player|GetPlayerPawn 0)))
      (if (Variables|/Game/FirstPerson/Blueprints/BP_FirstPersonCharacter.BP_FirstPersonCharacter_C|GetSprintGranted? _asbp_first_person_character)
        (if (== (Variables|/Game/FirstPerson/Blueprints/BP_FirstPersonCharacter.BP_FirstPersonCharacter_C|GetSprintActiveTime _asbp_first_person_character) (Variables|Default|GetSprintUpgradeTime))
          (|PlayerAlreadyHasUpgrade)
          (else
            (|GrantFlashLightUpgrade _asbp_first_person_character (Variables|Default|GetSprintUpgradeTime))))
        (else
          (|PlayerHasNoFlashlight))))))

(fn ConstructionScript)