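; Paired door and key actor that lets the player pick up a key and use the door to load another level.
; Trigger overlaps show locked, unlocked or pickup prompts; ActivateDoor reveals the sprite key and enables its pickup.
; Use/Pickup grants the key with a fading hint, or at the door freezes the player before opening the level.
; Tick enables input only while active and overlapped, and turns the key toward the camera.
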(event OnComponentBeginOverlap(DoorTrigger)
  (params (OverlappedComponent :type Primitive%20Component%20Object%20Reference) (OtherActor :type Actor%20Object%20Reference) (OtherComp :type Primitive%20Component%20Object%20Reference) (OtherBodyIndex :type Integer) (bFromSweep :type Boolean) (SweepResult :type Hit%20Result%20Structure%20%28by%20ref%29))
  ;[1 1 1] Show Door UI Prompt. Changes if player has a key to an unlocked prompt
  (Utilities|Casting|CastToBP_FirstPersonCharacter OtherActor)
  (Variables|Default|SetIsOverlapDoor? true)
  (if (Variables|Default|GetHasKey?)
    (Utilities|IsValid (Variables|LockAndKeyVariables|GetPickupPrompt)
      (:Is%20Not%20Valid
        (bind _returnvalue (UserInterface|CreateWidget "/Game/ClosingCall/UI/PickupPrompt.PickupPrompt_C"))
        (bind _output_get (Variables|LockAndKeyVariables|SetPickupPrompt _returnvalue))
        (Variables|/Game/ClosingCall/UI/PickupPrompt.PickupPrompt_C|SetPromptText _output_get (Utilities|Text|ToText(String) (Utilities|String|Append (Variables|LockAndKeyVariables|GetDoorUnlockedPromptText) (Variables|LockAndKeyVariables|GetDoorName))))
        (UserInterface|Viewport|AddtoViewport _output_get 0)))
    (else
      (Utilities|IsValid (Variables|LockAndKeyVariables|GetPickupPrompt)
        (:Is%20Not%20Valid
          (bind _returnvalue_2 (UserInterface|CreateWidget "/Game/ClosingCall/UI/PickupPrompt.PickupPrompt_C"))
          (bind _output_get_2 (Variables|LockAndKeyVariables|SetPickupPrompt _returnvalue_2))
          (Variables|/Game/ClosingCall/UI/PickupPrompt.PickupPrompt_C|SetPromptText _output_get_2 (Variables|LockAndKeyVariables|GetDoorLockedPromptText))
          (UserInterface|Viewport|AddtoViewport _output_get_2 0))))))

(event OnComponentEndOverlap(DoorTrigger)
  (params (OverlappedComponent :type Primitive%20Component%20Object%20Reference) (OtherActor :type Actor%20Object%20Reference) (OtherComp :type Primitive%20Component%20Object%20Reference) (OtherBodyIndex :type Integer))
  ;[1 1 1] Remove Door Prompt UI when player stops overlapping it
  (Utilities|Casting|CastToBP_FirstPersonCharacter OtherActor)
  (Variables|Default|SetIsOverlapDoor? false)
  (Utilities|IsValid (Variables|LockAndKeyVariables|GetPickupPrompt)
    (:Is%20Valid
      (Widget|RemovefromParent (Variables|LockAndKeyVariables|GetPickupPrompt))
      (Variables|LockAndKeyVariables|SetPickupPrompt 0))))

(event OnComponentBeginOverlap(KeyPickupTrig)
  (params (OverlappedComponent :type Primitive%20Component%20Object%20Reference) (OtherActor :type Actor%20Object%20Reference) (OtherComp :type Primitive%20Component%20Object%20Reference) (OtherBodyIndex :type Integer) (bFromSweep :type Boolean) (SweepResult :type Hit%20Result%20Structure%20%28by%20ref%29))
  ;[1 1 1] Create and Destroy UI Prompt for when player overlaps key
  (Utilities|Casting|CastToBP_FirstPersonCharacter OtherActor)
  (if (Variables|LockandKeyVariables|GetIsActive?)
    (Variables|Default|SetIsOverlapKey? true)
    (Utilities|IsValid (Variables|LockAndKeyVariables|GetPickupPrompt)
      (:Is%20Not%20Valid
        (bind _returnvalue (UserInterface|CreateWidget "/Game/ClosingCall/UI/PickupPrompt.PickupPrompt_C"))
        (bind _output_get (Variables|LockAndKeyVariables|SetPickupPrompt _returnvalue))
        (Variables|/Game/ClosingCall/UI/PickupPrompt.PickupPrompt_C|SetPromptText _output_get (Utilities|Text|ToText(String) (Utilities|String|Append (Variables|LockAndKeyVariables|GetKeyPickupPromptText) (Variables|LockAndKeyVariables|GetKeyName))))
        (UserInterface|Viewport|AddtoViewport _output_get 0)))))

(event OnComponentEndOverlap(KeyPickupTrig)
  (params (OverlappedComponent :type Primitive%20Component%20Object%20Reference) (OtherActor :type Actor%20Object%20Reference) (OtherComp :type Primitive%20Component%20Object%20Reference) (OtherBodyIndex :type Integer))
  ;[1 1 1] Create and Destroy UI Prompt for when player overlaps key
  (Utilities|Casting|CastToBP_FirstPersonCharacter OtherActor)
  (if (Variables|LockandKeyVariables|GetIsActive?)
    (Variables|Default|SetIsOverlapKey? false)
    (Utilities|IsValid (Variables|LockAndKeyVariables|GetPickupPrompt)
      (:Is%20Valid
        (Widget|RemovefromParent (Variables|LockAndKeyVariables|GetPickupPrompt))
        (Variables|LockAndKeyVariables|SetPickupPrompt 0)))))

(event Custom|ActivateDoor
  ;[1 1 1] Activate Door Event
  (Variables|LockandKeyVariables|SetIsActive? true)
  (Rendering|SetVisibility (Variables|Default|GetKeyPaperSprite) true false))

(event EventTick
  (params (DeltaSeconds :type Float%20%28single-precision%29))
  (bind _keypickup (Variables|Default|GetKeyPickup))
  (bind _playerref (Variables|Default|GetPlayerRef))
  ;[1 1 1] Enable and Disable Input depending on if player overlaps
  (Utilities|FlowControl|Sequence
    (:then_0
      (if (and (or (Variables|Default|GetIsOverlapDoor?) (Variables|Default|GetIsOverlapKey?)) (Variables|LockandKeyVariables|GetIsActive?))
        (Input|EnableInput _playerref)
        (else
          (Input|DisableInput _playerref))))
    (:then_1
      ;[1 1 1] Always face player
      (Utilities|IsValid _keypickup
        (:Is%20Valid
          (Transformation|SetRelativeRotation _keypickup (Math|Rotator|MakeRotfromX (- (Transformation|GetWorldLocation _keypickup) (Transformation|GetActorLocation (Game|GetPlayerCameraManager 0)))) false false))))))

(event EventBeginPlay
  ;[1 1 1] Get Player Ref
  (Variables|Default|SetPlayerRef (Game|GetPlayerController 0))
  (Rendering|Components|Sprite|SetSprite (Variables|Default|GetKeyPaperSprite) (Variables|LockAndKeyVariables|GetKeySprite))
  (if (not (Variables|LockandKeyVariables|GetIsActive?))
    (Rendering|SetVisibility (Variables|Default|GetKeyPaperSprite) false false)))

(event Input|ActionEvents|InputActionUse/Pickup
  (params (Key :type Key%20Structure :default "None"))
  ;[1 1 1] Handle Key Pickup and Level Transition
  (:Pressed
    (if (and (Variables|Default|GetIsOverlapKey?) (Variables|LockandKeyVariables|GetIsActive?))
      (Variables|Default|SetHasKey? true)
      (bind _returnvalue (UserInterface|CreateWidget "/Game/ClosingCall/UI/PlayerHint.PlayerHint_C"))
      (Variables|/Game/ClosingCall/UI/PlayerHint.PlayerHint_C|SetPromptText _returnvalue (Utilities|Text|ToText(String) (Utilities|String|Append (Variables|LockAndKeyVariables|GetPickedUpPrompt) (Variables|LockAndKeyVariables|GetKeyName))))
      (UserInterface|Viewport|AddtoViewport _returnvalue 0)
      (UserInterface|Animation|PlayAnimation _returnvalue (Variables|/Game/ClosingCall/UI/PlayerHint.PlayerHint_C|GetFadeOut _returnvalue) 0.0 1 "Forward" 1.0 false)
      (Components|DestroyComponent (Variables|Default|GetKeyPickup))
      (Components|DestroyComponent (Variables|Default|GetBillboard))
      (Components|DestroyComponent (Variables|Default|GetKeyPickupTrig))
      (Components|DestroyComponent (Variables|Default|GetKeyPaperSprite))
      (Utilities|IsValid (Variables|LockAndKeyVariables|GetPickupPrompt)
        (:Is%20Valid
          (Widget|RemovefromParent (Variables|LockAndKeyVariables|GetPickupPrompt))
          (Variables|LockAndKeyVariables|SetPickupPrompt 0)
          (Utilities|FlowControl|Delay 5.0)
          (Widget|RemovefromParent _returnvalue)))
      (elif (and (Variables|Default|GetIsOverlapDoor?) (Variables|Default|GetHasKey?))
        (bind _returnvalue_2 (Actor|GetActorOfClass "/Game/FirstPerson/Blueprints/BP_FirstPersonCharacter.BP_FirstPersonCharacter_C"))
        (UserInterface|Animation|PlayAnimation (Variables|/Game/FirstPerson/Blueprints/BP_FirstPersonCharacter.BP_FirstPersonCharacter_C|GetCenterAimingDot _returnvalue_2) (Variables|/Game/ClosingCall/UI/CenterAimingDot.CenterAimingDot_C|GetFadeIn (Variables|/Game/FirstPerson/Blueprints/BP_FirstPersonCharacter.BP_FirstPersonCharacter_C|GetCenterAimingDot _returnvalue_2)) 0.0 1 "Forward" 1.0 false)
        (Pawn|Components|CharacterMovement|DisableMovement (Variables|/Script/Engine.Character|GetCharacterMovement _returnvalue_2))
        (Utilities|FlowControl|Delay 1.0)
        (Game|OpenLevel(byObjectReference) (Variables|LockAndKeyVariables|GetLevel))))))

(fn ConstructionScript)