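; Paranormal event actor that throws a physics item when the first-person character walks into its trigger.
; The overlap applies a force to ItemToLaunch along the Arrow's forward vector, destroys the trigger so it fires once, and plays a plastic box hit sound.
; Item collisions replay that sound only when the hit actor differs from the last one.
; A one-second delay after BeginPlay arms both trigger and hit sounds.
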(event OnComponentHit(ItemToLaunch)
  (params (HitComponent :type Primitive%20Component%20Object%20Reference) (OtherActor :type Actor%20Object%20Reference) (OtherComp :type Primitive%20Component%20Object%20Reference) (NormalImpulse :type Vector :default "0, 0, 0") (Hit :type Hit%20Result%20Structure%20%28by%20ref%29))
  (if (Variables|Default|GetIsActive)
    (bind _output_get (Variables|Default|SetOther%20Actor OtherActor))
    (if (not (== (Variables|Default|GetLastActor) _output_get))
      (Variables|Default|SetLastActor _output_get)
      (Audio|PlaySoundatLocation "/Game/ClosingCall/Sound/PlasticBox/PlasticBoxHit.PlasticBoxHit" (Transformation|GetWorldLocation (Variables|Default|GetItemToLaunch)) "0, 0, 0" 1.0 1.0 0.0 "/Game/ClosingCall/Sound/CCSoundAttenuation.CCSoundAttenuation" 0 0 0))))

(event OnComponentBeginOverlap(Trigger)
  (params (OverlappedComponent :type Primitive%20Component%20Object%20Reference) (OtherActor :type Actor%20Object%20Reference) (OtherComp :type Primitive%20Component%20Object%20Reference) (OtherBodyIndex :type Integer) (bFromSweep :type Boolean) (SweepResult :type Hit%20Result%20Structure%20%28by%20ref%29))
  (if (Variables|Default|GetIsActive)
    (Utilities|Casting|CastToBP_FirstPersonCharacter OtherActor)
    (Physics|AddForce (Variables|Default|GetItemToLaunch) (* (Math|Vector|GetForwardVector (Variables|Default|GetArrow)) (Variables|Default|GetLaunchForce)) "None" false)
    (Components|DestroyComponent (Variables|Default|GetTrigger))
    (Audio|PlaySoundatLocation "/Game/ClosingCall/Sound/PlasticBox/PlasticBoxHit.PlasticBoxHit" (Transformation|GetWorldLocation (Variables|Default|GetItemToLaunch)) "0, 0, 0" 1.0 1.0 0.0 "/Game/ClosingCall/Sound/CCSoundAttenuation.CCSoundAttenuation" 0 0 0)))

(event EventBeginPlay
  (Utilities|FlowControl|Delay 1.0)
  (Variables|Default|SetIsActive true))

(event EventTick
  (params (DeltaSeconds :type Float%20%28single-precision%29)))

(fn ConstructionScript)