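; BP_Cable is a configurable cable actor that builds itself along a spline in the construction script, with no runtime logic.
; Each spline segment gets a spline mesh matched to its points and tangents and scaled by cable thickness.
; Optional start and end connector meshes align to the spline tangents, with adjustable roll; the end one reuses the last segment's stored values.
; One dynamic material instance, shared by all segments, applies the cable color.
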(event EventBeginPlay)

(event Collision|EventActorBeginOverlap
  (params (OtherActor :type Actor%20Object%20Reference)))

(event EventTick
  (params (DeltaSeconds :type Float%20%28single-precision%29)))

(fn ConstructionScript
  (bind _output_get (LocalVariables|SetPoints (- (Spline|GetNumberOfSplinePoints (Variables|Default|GetSpline)) 1)))
  (for _index (range 0 _output_get)
    (bind _output_get_2 (LocalVariables|SetIndex _index))
    (if (< _output_get_2 (LocalVariables|GetPoints))
      (|CreateSplineMeshAlignedToSpline)))
  (Utilities|FlowControl|Sequence
    (:then_0
      (|AddStartConnectorMesh))
    (:then_1
      (|AddEndConnectorMesh))
    (:then_2
      (|RotateConnectorMeshes))
    (:then_3
      (|SetDynamicMaterial))))